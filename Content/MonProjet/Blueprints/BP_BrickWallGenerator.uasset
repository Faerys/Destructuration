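; Actor that builds a brick wall of BP_Brick actors when the player presses Use inside its trigger box.
; BeginPlay derives the first brick position from BordureAvant and computes row and column counts from wall and brick dimensions.
; Box overlaps toggle input; nested loops spawn bricks, shifting every other row half a brick for a staggered bond.
; A ForLoopWithDelay macro is defined, but the generation loops shown run without delay.
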(event `self.ReceiveBeginPlay`
  (bind (_returnvalue_x _returnvalue_y _returnvalue_z) (`KismetMathLibrary.BreakVector` (`SceneComponent.K2_GetComponentLocation` (`self.BordureAvant`))))
  ;[0.4177 1 0.9] Initialisation
  (set `self.PositionDeLaPremiereBrique` (`KismetMathLibrary.MakeVector` (+ _returnvalue_x 50.0) (+ _returnvalue_y -150.0) (+ _returnvalue_z 0.5)))
  (bind _output_get (set `self.NombreDeBriqueEnLargeur` (`KismetMathLibrary.FTrunc` (/ (`self.LargeurDuMur`) (`self.LargeurDeLaBrique`)))))
  (`KismetSystemLibrary.PrintString` (`KismetStringLibrary.Conv_IntToString` _output_get))
  (bind _output_get_2 (set `self.NombreDeBriqueEnHauteur` (`KismetMathLibrary.FTrunc` (/ (`self.HauteurDuMur`) (`self.HauteurDeLaBrique`)))))
  (`KismetSystemLibrary.PrintString` (`KismetStringLibrary.Conv_IntToString` _output_get_2))
  (set `self.bDecalage` false))

(event `self.Box.OnComponentBeginOverlap`
  (params (OverlappedComponent :type "PrimitiveComponent Object Reference") (OtherActor :type "Actor Object Reference") (OtherComp :type "PrimitiveComponent Object Reference") (OtherBodyIndex :type Integer) (bFromSweep :type Boolean) (SweepResult :type "HitResult Structure (by ref)"))
  (`KismetSystemLibrary.PrintString` "Possibilité de construire le mur" true true (struct :`R` 0.226297 :`G` 1.0 :`A` 1.0))
  (`self.EnableInput` (`GameplayStatics.GetPlayerController` 0)))

(event `InputAction|kb_Use`
  (params (Key :type "Key Structure"))
  (bind _positiondelapremierebrique (`self.PositionDeLaPremiereBrique`))
  (bind _positiondelabriqueaposer (`self.PositionDeLaBriqueAPoser`))
  ;[1 0.4316 0.8227] Génération du mur
  (:`Pressed`
    ;;[1 1 1] Premiere boucle, gestion de la hauteur
    (for _index (range 1 (+ (`self.NombreDeBriqueEnHauteur`) 1))
      (if (`self.bDecalage`)
        (bind _returnvalue (+ (.z _positiondelapremierebrique) (* (- _index 1) (`self.HauteurDeLaBrique`))))
        (set `self.PositionDeLaBriqueAPoser` (`KismetMathLibrary.MakeVector` (.x _positiondelapremierebrique) (+ (.y _positiondelapremierebrique) (/ (`self.LargeurDeLaBrique`) 2.0)) _returnvalue))
        (else
          (set `self.PositionDeLaBriqueAPoser` (`KismetMathLibrary.MakeVector` (.x _positiondelapremierebrique) (.y _positiondelapremierebrique) _returnvalue))))
      ;;;[0.05673 0.3207 1] 2nd boucle, pour la largeur
      (for _ (range 1 (+ (`self.NombreDeBriqueEnLargeur`) 1))
        (`|SpawnActorFromClass` "/Game/MonProjet/Blueprints/BP_Brick.BP_Brick_C" (`KismetMathLibrary.MakeTransform` _positiondelabriqueaposer) "Undefined" "OverrideRootScale" null null)
        (set `self.PositionDeLaBriqueAPoser` (`KismetMathLibrary.MakeVector` (.x _positiondelabriqueaposer) (+ (.y _positiondelabriqueaposer) (`self.LargeurDeLaBrique`)) (.z _positiondelabriqueaposer))))
      (set `self.bDecalage` (not (`self.bDecalage`))))
    (`KismetSystemLibrary.PrintString` "Fin de la construction du mur" true true (struct :`R` 0.07169 :`G` 0.192708 :`B` 0.061613 :`A` 1.0))))

(event `self.Box.OnComponentEndOverlap`
  (params (OverlappedComponent :type "PrimitiveComponent Object Reference") (OtherActor :type "Actor Object Reference") (OtherComp :type "PrimitiveComponent Object Reference") (OtherBodyIndex :type Integer))
  (`KismetSystemLibrary.PrintString` "Impossibilité de construire le mur" true true (struct :`R` 0.205831 :`G` 1.0 :`A` 1.0))
  (`self.DisableInput` (`GameplayStatics.GetPlayerController` 0)))

(fn `UserConstructionScript`)