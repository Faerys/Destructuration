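; BP_MyProjectile_Bullet is a projectile that deals radial damage where it hits, then destroys itself.
; BeginPlay stores the spawn location for use when the Hit event fires.
; On hit, it prints the struck actor's name, applies damage and spawns a non-auto-destroying plasma emitter scaled by the damage radius.
; A line trace from spawn point to impact serves only as a timed debug drawing of the shot.
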(event `self.ReceiveHit`
  (params (MyComp :type "PrimitiveComponent Object Reference") (Other :type "Actor Object Reference") (OtherComp :type "PrimitiveComponent Object Reference") (bSelfMoved :type Boolean) (HitLocation :type "Vector Structure") (HitNormal :type "Vector Structure") (NormalImpulse :type "Vector Structure") (Hit :type "HitResult Structure (by ref)"))
  ;[0.7672 0.7396 1] Ajout d'un Radial Damage
  (`KismetSystemLibrary.PrintString` (`KismetSystemLibrary.GetObjectName` (`ActorComponent.GetOwner` OtherComp)) true true (`self.HitTextColor`) (`self.HitTextDuration`))
  (`GameplayStatics.ApplyRadialDamage` :`BaseDamage` (`self.BaseDamage`) :`Origin` HitLocation :`DamageRadius` (`self.DamageRadius`) :`DamageCauser` (`ActorComponent.GetOwner` MyComp) :`InstigatedByController` null)
  (`GameplayStatics.SpawnEmitterAtLocation` (`self.Part_PlasmaBall`) HitLocation (struct) (* (1.0 1.0 1.0) (`self.DamageRadius`)) false)
  (`KismetSystemLibrary.LineTraceSingle` :`Start` (stale `self.ReceiveBeginPlay` _output_get) :`End` HitLocation :`TraceChannel` "TraceTypeQuery1" :`DrawDebugType` "ForDuration" :`TraceColor` (struct :`G` 0.08703 :`B` 0.432292 :`A` 1.0))
  (`self.K2_DestroyActor`))

(event `self.ReceiveBeginPlay`
  ;[0.7672 0.7396 1] Ajout d'un Radial Damage
  ;;[0 0.2264 1] Start point for LineTraceByChannel
  (bind _output_get (set `self.LocN-1` (`self.K2_GetActorLocation`))))

(fn `UserConstructionScript`)