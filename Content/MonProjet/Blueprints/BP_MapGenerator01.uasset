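; BP_MapGenerator01 procedurally generates a walled floor arena beyond a Start component, with random brick obstacles and a local navigation grid.
; The Construction Script builds tiles, walls and grid when width and depth are non-zero; otherwise FloorConstruction and WallConstruction run on switch use.
; Pressing Use inside the switch's trigger box also spawns randomly scaled BP_ProceduralBricks within floor bounds, skipping unresolvable collisions.
; The pressed switch loses its glow, emits fireflies and bobs on Tick.
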(event `self.ReceiveBeginPlay`
  (bind _unitstandard (`self.UnitStandard`))
  (bind _returnvalue (* (`self.ProceduralFloor_Scale`) _unitstandard))
  (bind (_relativelocation_x _relativelocation_y _relativelocation_z) (`KismetMathLibrary.BreakVector` (`SceneComponent.RelativeLocation` (`self.SwitchButton`))))
  ;[1 1 1] Switch Button movement
  (bind _output_get (set `self.Z_SwitchButtonInitialLocation` _relativelocation_z))
  (set `self.Z_SwitchLocation` _output_get)
  (bind _returnvalue_2 (`PrimitiveComponent.CreateDynamicMaterialInstance` (`self.SwitchButton`) 0 "/Game/MonProjet/Materials/M_GlowSwitchButton.M_GlowSwitchButton" "None"))
  (set `self.DynamicMaterial_SwitchButton` _returnvalue_2)
  (`GameplayStatics.SpawnEmitterAtLocation` "/Game/Particles_Wind_Control_System/Particles/P_Fireflies.P_Fireflies" (`SceneComponent.K2_GetComponentLocation` (`self.SwitchButton`)) (struct) (0.2 0.2 0.2))
  (if (not (`self.FloorIsAlreadyBuilt`))
    (set `self.ProceduralFloorLocation_X_Offset` (+ (/ (* (`self.ProceduralFloor_Scale`) _unitstandard) 2.0) (`self.ProceduralFloorLocation_X_Offset`)))
    (set `self.ProceduralFloorLocation_Y_Offset` (+ (/ (* (`self.Width_ProceduralFloor`) _returnvalue) -2.0) (/ _returnvalue 2.0)))))

(event `self.ReceiveTick`
  (params (DeltaSeconds :type "Float (single-precision)"))
  (bind (_relativelocation_x _relativelocation_y _relativelocation_z) (`KismetMathLibrary.BreakVector` (`SceneComponent.RelativeLocation` (`self.SwitchButton`))))
  ;[1 1 1] Switch Button movement
  (if (`self.ButtonPressed?`)
    (if (`self.SwitchGoesUp?`)
      (set `self.Z_SwitchLocation` (+ (`self.Z_SwitchLocation`) (`self.SwitchSpeed`)))
      (else
        (set `self.Z_SwitchLocation` (- (`self.Z_SwitchLocation`) (`self.SwitchSpeed`)))))
    (`SceneComponent.K2_SetRelativeLocation` (`self.SwitchButton`) (`KismetMathLibrary.MakeVector` _relativelocation_x _relativelocation_y (`self.Z_SwitchLocation`)) false false)
    (if (and (>= (- (`self.Z_SwitchLocation`) (`self.Z_SwitchButtonInitialLocation`)) 5.0) (`self.SwitchGoesUp?`))
      (set `self.SwitchGoesUp?` false)
      (elif (and (>= (- (`self.Z_SwitchButtonInitialLocation`) (`self.Z_SwitchLocation`)) 5.0) (not (`self.SwitchGoesUp?`)))
        (set `self.SwitchGoesUp?` true)))))

(event `self.SwitchButton_BoxCol.OnComponentBeginOverlap`
  (params (OverlappedComponent :type "PrimitiveComponent Object Reference") (OtherActor :type "Actor Object Reference") (OtherComp :type "PrimitiveComponent Object Reference") (OtherBodyIndex :type Integer) (bFromSweep :type Boolean) (SweepResult :type "HitResult Structure (by ref)"))
  (if (not (`self.ButtonPressed?`))
    (`self.EnableInput` (`GameplayStatics.GetPlayerController` 0))
    (`SceneComponent.SetHiddenInGame` (`self.Text_PressF`) false false)))

(event `self.SwitchButton_BoxCol.OnComponentEndOverlap`
  (params (OverlappedComponent :type "PrimitiveComponent Object Reference") (OtherActor :type "Actor Object Reference") (OtherComp :type "PrimitiveComponent Object Reference") (OtherBodyIndex :type Integer))
  (`self.DisableInput` (`GameplayStatics.GetPlayerController` 0))
  (`SceneComponent.SetHiddenInGame` (`self.Text_PressF`) true false))

(event `InputAction|kb_Use`
  (params (Key :type "Key Structure"))
  (:`Pressed`
    (`self.SwitchAnimation`)
    (if (not (`self.FloorIsAlreadyBuilt`))
      ;[0 1 0.04794] Floor & Wall construction at runtime
      (`self.FloorConstruction`)
      (`self.WallConstruction`))
    ;[0 1 0.01348] Obstacles construction
    (`self.ObstaclesConstruction`)))

(fn `FloorConstruction`
  (bind _proceduralfloor_scale (`self.ProceduralFloor_Scale`))
  (bind (_returnvalue_x _returnvalue_y _returnvalue_z) (`KismetMathLibrary.BreakVector` (`SceneComponent.K2_GetComponentLocation` (`self.Start`))))
  (for _ (range 1 (+ (`self.Depth_ProceduralFloor`) 1))
    (for _ (range 1 (+ (`self.Width_ProceduralFloor`) 1))
      (`AddComponent|NODE_AddStaticMeshComponent-18` :`RelativeTransform` (`KismetMathLibrary.MakeTransform` (`KismetMathLibrary.MakeVector` (+ (`self.ProceduralFloorLocation_X`) (`self.ProceduralFloorLocation_X_Offset`)) (+ (`self.ProceduralFloorLocation_Y`) (`self.ProceduralFloorLocation_Y_Offset`)) _returnvalue_z) (struct) (`KismetMathLibrary.MakeVector` _proceduralfloor_scale _proceduralfloor_scale 1.0)))
      (set `self.ProceduralFloorLocation_Y` (+ (`self.ProceduralFloorLocation_Y`) (* (`self.ProceduralFloor_Scale`) (`self.UnitStandard`)))))
    (set `self.ProceduralFloorLocation_X` (+ (`self.ProceduralFloorLocation_X`) (* (`self.ProceduralFloor_Scale`) (`self.UnitStandard`))))
    (set `self.ProceduralFloorLocation_Y` 0.0)))

(fn `ObstaclesConstruction`
  (bind _returnvalue (`KismetMathLibrary.RandomFloatInRange` 0.2 2.0))
  (bind _unitstandard (`self.UnitStandard`))
  (bind (_returnvalue_x _returnvalue_y _returnvalue_z) (`KismetMathLibrary.BreakVector` (`SceneComponent.K2_GetComponentLocation` (`self.Start`))))
  (bind _returnvalue_2 (/ (* (`self.ProceduralBrick_Scale_X`) _unitstandard) 2.0))
  (bind _returnvalue_3 (/ (* (`self.ProceduralBrick_Scale_Y`) _unitstandard) 2.0))
  (bind _returnvalue_4 (- (`self.ProceduralFloorLocation_Y_Offset`) (/ (* (`self.ProceduralFloor_Scale`) _unitstandard) 2.0)))
  (bind _returnvalue_5 (- (`self.ProceduralFloorLocation_X_Offset`) (/ (* (`self.ProceduralFloor_Scale`) _unitstandard) 2.0)))
  (for _ (range 1 (+ (`self.NumberOfObstacle`) 1))
    (set `self.ProceduralBrick_Scale_X` _returnvalue)
    (set `self.ProceduralBrick_Scale_Y` _returnvalue)
    (set `self.ProceduralBrick_Scale_Z` _returnvalue)
    (`|SpawnActorFromClass` "/Game/MonProjet/Blueprints/BP_ProceduralBrick.BP_ProceduralBrick_C" (`KismetMathLibrary.MakeTransform` (`KismetMathLibrary.MakeVector` (`KismetMathLibrary.RandomFloatInRange` (+ _returnvalue_5 _returnvalue_2) (- (+ _returnvalue_5 (* (`self.ProceduralFloor_Scale`) 100.0 (`KismetMathLibrary.Conv_IntToDouble` (`self.Depth_ProceduralFloor`)))) _returnvalue_2)) (`KismetMathLibrary.RandomFloatInRange` (+ _returnvalue_4 _returnvalue_3) (- (+ _returnvalue_4 (* (`self.ProceduralFloor_Scale`) 100.0 (`KismetMathLibrary.Conv_IntToDouble` (`self.Width_ProceduralFloor`)))) _returnvalue_3)) (+ _returnvalue_z (/ (* (`self.ProceduralBrick_Scale_Z`) (`self.UnitStandard`)) 2.0))) (struct) (`KismetMathLibrary.MakeVector` (`self.ProceduralBrick_Scale_X`) (`self.ProceduralBrick_Scale_Y`) (`self.ProceduralBrick_Scale_Z`))) "AdjustIfPossibleButDontSpawnIfColliding" "OverrideRootScale" null null)))

(fn `SwitchAnimation`
  (bind _switchbutton (`self.SwitchButton`))
  (bind _switchbutton_2 (`self.SwitchButton`))
  (bind (_relativelocation_x _relativelocation_y) (`KismetMathLibrary.BreakVector` (`SceneComponent.RelativeLocation` _switchbutton)))
  (`SceneComponent.K2_SetRelativeLocation` _switchbutton (`KismetMathLibrary.MakeVector` _relativelocation_x _relativelocation_y (+ (`self.Z_SwitchLocation`) 1.0)) false false)
  (`MaterialInstanceDynamic.SetScalarParameterValue` (`self.DynamicMaterial_SwitchButton`) "Glow" 0.0)
  (`GameplayStatics.SpawnEmitterAtLocation` "/Game/Particles_Wind_Control_System/Particles/P_Fireflies.P_Fireflies" (`SceneComponent.K2_GetComponentLocation` _switchbutton_2) (struct) (0.2 0.2 0.2))
  (set `self.ButtonPressed?` true)
  (bind _output_get (set `self.Z_SwitchButtonInitialLocation` (.z (`SceneComponent.RelativeLocation` _switchbutton_2))))
  (set `self.Z_SwitchLocation` _output_get))

(fn `UserConstructionScript`
  (bind (_returnvalue_x _returnvalue_y _returnvalue_z) (`KismetMathLibrary.BreakVector` (`self.K2_GetActorLocation`)))
  (bind _start (`self.Start`))
  (bind _unitstandard (`self.UnitStandard`))
  (bind _proceduralfloor_scale (`self.ProceduralFloor_Scale`))
  (bind _wallwidth_scale (`self.WallWidth_Scale`))
  (bind _start_2 (`self.Start`))
  (bind _wallheight_scale (`self.WallHeight_Scale`))
  (bind _wallwidth_scale_2 (`self.WallWidth_Scale`))
  (bind _wallheight_scale_2 (`self.WallHeight_Scale`))
  (bind _wallwidth_scale_3 (`self.WallWidth_Scale`))
  (bind _proceduralfloor_scale_2 (`self.ProceduralFloor_Scale`))
  (bind _unitstandard_2 (`self.UnitStandard`))
  (bind (_returnvalue_x_2 _returnvalue_y_2 _returnvalue_z_2) (`KismetMathLibrary.BreakVector` (`SceneComponent.K2_GetComponentLocation` (`self.Start`))))
  (bind _returnvalue_x_3 (`KismetMathLibrary.BreakVector` (`SceneComponent.K2_GetComponentLocation` _start)))
  (bind (_returnvalue_x_4 _returnvalue_y_3 _returnvalue_z_3) (`KismetMathLibrary.BreakVector` (`SceneComponent.K2_GetComponentLocation` _start_2)))
  (bind _returnvalue_x_5 (`KismetMathLibrary.BreakVector` (`SceneComponent.K2_GetComponentScale` _start_2)))
  (bind _returnvalue_x_6 (`KismetMathLibrary.BreakVector` (`SceneComponent.K2_GetComponentScale` _start)))
  (bind _returnvalue (* (`self.Depth_ProceduralFloor`) (`self.ProceduralFloor_Scale`)))
  (bind (_returnvalue_x_7 _returnvalue_y_4) (`KismetMathLibrary.BreakVector` (`SceneComponent.K2_GetComponentScale` (`self.Start`))))
  (bind _returnvalue_x_8 (`KismetMathLibrary.BreakVector` (`SceneComponent.K2_GetComponentScale` (`self.Start`))))
  (bind _returnvalue_2 (* _unitstandard (`self.ProceduralFloor_Scale`)))
  (bind _returnvalue_3 (/ _returnvalue_2 2.0))
  (bind _returnvalue_4 (* (`KismetMathLibrary.Conv_IntToDouble` (`self.Depth_ProceduralFloor`)) (`self.UnitStandard`) (`self.ProceduralFloor_Scale`)))
  (bind _returnvalue_5 (/ (* (`KismetMathLibrary.Conv_IntToDouble` (`self.Width_ProceduralFloor`)) (`self.ProceduralFloor_Scale`) (`self.UnitStandard`)) 2.0))
  (bind _returnvalue_6 (+ _returnvalue_z_3 (/ (* (`self.UnitStandard`) (`self.WallHeight_Scale`)) 2.0)))
  (bind _returnvalue_7 (/ (- (- (* (`self.Width_ProceduralFloor`) (`self.ProceduralFloor_Scale`)) _returnvalue_y_4) (`self.WallWidth_Scale`)) 2.0))
  (bind _returnvalue_8 (+ (/ (* _returnvalue_x_5 (`self.UnitStandard`)) 2.0) _returnvalue_x_4))
  (bind _returnvalue_9 (+ (/ _returnvalue_4 2.0) _returnvalue_8))
  (bind _returnvalue_10 (* (/ (+ _returnvalue_7 _returnvalue_y_4) 2.0) (`self.UnitStandard`)))
  (if (or (== (`self.Width_ProceduralFloor`) 0) (== (`self.Depth_ProceduralFloor`) 0))
    (set `self.FloorIsAlreadyBuilt` false)
    (else
      (set `self.ProceduralFloorLocation_X_Offset` (+ (+ _returnvalue_x_3 (/ (* _returnvalue_x_6 _unitstandard) 2.0)) _returnvalue_3))
      (set `self.ProceduralFloorLocation_Y_Offset` (- _returnvalue_3 (/ (* _returnvalue_2 (`KismetMathLibrary.Conv_IntToDouble` (`self.Width_ProceduralFloor`))) 2.0)))
      (for _ (range 1 (+ (`self.Depth_ProceduralFloor`) 1))
        (for _ (range 1 (+ (`self.Width_ProceduralFloor`) 1))
          (`AddComponent|NODE_AddStaticMeshComponent-7` :`RelativeTransform` (`KismetMathLibrary.MakeTransform` (`KismetMathLibrary.MakeVector` (+ (`self.ProceduralFloorLocation_X`) (`self.ProceduralFloorLocation_X_Offset`)) (+ (`self.ProceduralFloorLocation_Y`) (`self.ProceduralFloorLocation_Y_Offset`)) _returnvalue_z_2) (struct) (`KismetMathLibrary.MakeVector` _proceduralfloor_scale _proceduralfloor_scale 1.0)))
          (set `self.ProceduralFloorLocation_Y` (+ (`self.ProceduralFloorLocation_Y`) (* (`self.ProceduralFloor_Scale`) (`self.UnitStandard`)))))
        (set `self.ProceduralFloorLocation_X` (+ (`self.ProceduralFloorLocation_X`) (* (`self.ProceduralFloor_Scale`) (`self.UnitStandard`))))
        (set `self.ProceduralFloorLocation_Y` 0.0))
      (set `self.FloorIsAlreadyBuilt` true)
      (`AddComponent|NODE_AddStaticMeshComponent-8` :`RelativeTransform` (`KismetMathLibrary.MakeTransform` (`KismetMathLibrary.MakeVector` _returnvalue_8 (+ _returnvalue_10 _returnvalue_y_3) _returnvalue_6) (struct) (`KismetMathLibrary.MakeVector` _wallwidth_scale _returnvalue_7 _wallheight_scale)))
      (`AddComponent|NODE_AddStaticMeshComponent-9` :`RelativeTransform` (`KismetMathLibrary.MakeTransform` (`KismetMathLibrary.MakeVector` _returnvalue_8 (+ (* _returnvalue_10 -1.0) _returnvalue_y_3) _returnvalue_6) (struct) (`KismetMathLibrary.MakeVector` _wallwidth_scale _returnvalue_7 _wallheight_scale)))
      (`AddComponent|NODE_AddStaticMeshComponent-10` :`RelativeTransform` (`KismetMathLibrary.MakeTransform` (`KismetMathLibrary.MakeVector` (+ _returnvalue_4 _returnvalue_8) _returnvalue_y_3 _returnvalue_6) (struct) (`KismetMathLibrary.MakeVector` _wallwidth_scale_2 (- (* (`self.Width_ProceduralFloor`) (`self.ProceduralFloor_Scale`)) _wallwidth_scale_2) _wallheight_scale_2)))
      (`AddComponent|NODE_AddStaticMeshComponent-11` :`RelativeTransform` (`KismetMathLibrary.MakeTransform` (`KismetMathLibrary.MakeVector` _returnvalue_9 _returnvalue_5 _returnvalue_6) (struct) (`KismetMathLibrary.MakeVector` _returnvalue _wallwidth_scale_3 _wallheight_scale_2)))
      (`AddComponent|NODE_AddStaticMeshComponent-12` :`RelativeTransform` (`KismetMathLibrary.MakeTransform` (`KismetMathLibrary.MakeVector` _returnvalue_9 (* _returnvalue_5 -1.0) _returnvalue_6) (struct) (`KismetMathLibrary.MakeVector` _returnvalue _wallwidth_scale_3 _wallheight_scale_2)))
      (`NavLocalGridManager.AddLocalNavigationGridForBox` (`KismetMathLibrary.MakeVector` (/ (* 0.0 (+ _returnvalue_x_8 (* (`self.Depth_ProceduralFloor`) (`self.ProceduralFloor_Scale`)))) 2.0) 0.0 _returnvalue_z) (`KismetMathLibrary.MakeVector` (* (`KismetMathLibrary.Conv_IntToDouble` (`self.Width_ProceduralFloor`)) _proceduralfloor_scale_2 _unitstandard_2) (* _proceduralfloor_scale_2 _unitstandard_2 (`KismetMathLibrary.Conv_IntToDouble` (`self.Depth_ProceduralFloor`))) 1.0) (struct) 5 10.0))))

(fn `WallConstruction`
  (bind (_returnvalue_x _returnvalue_y _returnvalue_z) (`KismetMathLibrary.BreakVector` (`self.K2_GetActorLocation`)))
  (bind _wallwidth_scale (`self.WallWidth_Scale`))
  (bind _start (`self.Start`))
  (bind _wallheight_scale (`self.WallHeight_Scale`))
  (bind _wallwidth_scale_2 (`self.WallWidth_Scale`))
  (bind _wallheight_scale_2 (`self.WallHeight_Scale`))
  (bind _wallwidth_scale_3 (`self.WallWidth_Scale`))
  (bind _proceduralfloor_scale (`self.ProceduralFloor_Scale`))
  (bind _unitstandard (`self.UnitStandard`))
  (bind (_returnvalue_x_2 _returnvalue_y_2 _returnvalue_z_2) (`KismetMathLibrary.BreakVector` (`SceneComponent.K2_GetComponentLocation` _start)))
  (bind _returnvalue_x_3 (`KismetMathLibrary.BreakVector` (`SceneComponent.K2_GetComponentScale` _start)))
  (bind _returnvalue (* (`self.Depth_ProceduralFloor`) (`self.ProceduralFloor_Scale`)))
  (bind (_returnvalue_x_4 _returnvalue_y_3) (`KismetMathLibrary.BreakVector` (`SceneComponent.K2_GetComponentScale` (`self.Start`))))
  (bind _returnvalue_x_5 (`KismetMathLibrary.BreakVector` (`SceneComponent.K2_GetComponentScale` (`self.Start`))))
  (bind _returnvalue_2 (* (`KismetMathLibrary.Conv_IntToDouble` (`self.Depth_ProceduralFloor`)) (`self.UnitStandard`) (`self.ProceduralFloor_Scale`)))
  (bind _returnvalue_3 (/ (* (`KismetMathLibrary.Conv_IntToDouble` (`self.Width_ProceduralFloor`)) (`self.ProceduralFloor_Scale`) (`self.UnitStandard`)) 2.0))
  (bind _returnvalue_4 (+ _returnvalue_z_2 (/ (* (`self.UnitStandard`) (`self.WallHeight_Scale`)) 2.0)))
  (bind _returnvalue_5 (/ (- (- (* (`self.Width_ProceduralFloor`) (`self.ProceduralFloor_Scale`)) _returnvalue_y_3) (`self.WallWidth_Scale`)) 2.0))
  (bind _returnvalue_6 (+ (/ (* _returnvalue_x_3 (`self.UnitStandard`)) 2.0) _returnvalue_x_2))
  (bind _returnvalue_7 (+ (/ _returnvalue_2 2.0) _returnvalue_6))
  (bind _returnvalue_8 (* (/ (+ _returnvalue_5 _returnvalue_y_3) 2.0) (`self.UnitStandard`)))
  (`AddComponent|NODE_AddStaticMeshComponent-13` :`RelativeTransform` (`KismetMathLibrary.MakeTransform` (`KismetMathLibrary.MakeVector` _returnvalue_6 (+ _returnvalue_8 _returnvalue_y_2) _returnvalue_4) (struct) (`KismetMathLibrary.MakeVector` _wallwidth_scale _returnvalue_5 _wallheight_scale)))
  (`AddComponent|NODE_AddStaticMeshComponent-14` :`RelativeTransform` (`KismetMathLibrary.MakeTransform` (`KismetMathLibrary.MakeVector` _returnvalue_6 (+ (* _returnvalue_8 -1.0) _returnvalue_y_2) _returnvalue_4) (struct) (`KismetMathLibrary.MakeVector` _wallwidth_scale _returnvalue_5 _wallheight_scale)))
  (`AddComponent|NODE_AddStaticMeshComponent-15` :`RelativeTransform` (`KismetMathLibrary.MakeTransform` (`KismetMathLibrary.MakeVector` (+ _returnvalue_2 _returnvalue_6) _returnvalue_y_2 _returnvalue_4) (struct) (`KismetMathLibrary.MakeVector` _wallwidth_scale_2 (- (* (`self.Width_ProceduralFloor`) (`self.ProceduralFloor_Scale`)) _wallwidth_scale_2) _wallheight_scale_2)))
  (`AddComponent|NODE_AddStaticMeshComponent-16` :`RelativeTransform` (`KismetMathLibrary.MakeTransform` (`KismetMathLibrary.MakeVector` _returnvalue_7 _returnvalue_3 _returnvalue_4) (struct) (`KismetMathLibrary.MakeVector` _returnvalue _wallwidth_scale_3 _wallheight_scale_2)))
  (`AddComponent|NODE_AddStaticMeshComponent-17` :`RelativeTransform` (`KismetMathLibrary.MakeTransform` (`KismetMathLibrary.MakeVector` _returnvalue_7 (* _returnvalue_3 -1.0) _returnvalue_4) (struct) (`KismetMathLibrary.MakeVector` _returnvalue _wallwidth_scale_3 _wallheight_scale_2)))
  (`NavLocalGridManager.AddLocalNavigationGridForBox` (`KismetMathLibrary.MakeVector` (/ (* (`self.UnitStandard`) (+ _returnvalue_x_5 (* (`self.Depth_ProceduralFloor`) (`self.ProceduralFloor_Scale`)))) 2.0) 0.0 _returnvalue_z) (`KismetMathLibrary.MakeVector` (* (`KismetMathLibrary.Conv_IntToDouble` (`self.Width_ProceduralFloor`)) _proceduralfloor_scale _unitstandard) (* _proceduralfloor_scale _unitstandard (`KismetMathLibrary.Conv_IntToDouble` (`self.Depth_ProceduralFloor`))) 1.0) (struct) 5 10.0))