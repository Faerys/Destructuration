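; Twin spotlight actor whose shared color continuously cycles through hues.
; The construction script mirrors both lights across Y from gap and height, using arctangent to pitch them toward the actor origin plus a projection offset.
; Each Tick, RGBRotator runs a six-state machine that ramps one channel by a fixed, frame-rate-dependent step, then applies the color to both lights.
; Its Blue and Green variable names are swapped relative to the actual G and B channels.
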(event `self.ReceiveTick`
  (params (DeltaSeconds :type "Float (single-precision)"))
  (bind _lightcolor (`self.LightColor`))
  (bind _linear_color_output (`self.RGB_Rotator` (`self.LightColor`)))
  (set `self.LightColor` _linear_color_output)
  (`LightComponent.SetLightColor` (`self.SpotLight01`) _lightcolor true)
  (`LightComponent.SetLightColor` (`self.SpotLight02`) _lightcolor true))

(fn `RGB_Rotator`
  (params (`Linear Color Input` :type "LinearColor Structure"))
  (returns (`Linear Color Output` :type "LinearColor Structure"))
  (locals (_RedColor :type "Float (double-precision)" :default 255.0) (_BlueColor :type "Float (double-precision)") (_GreenColor :type "Float (double-precision)") (_ColorModifier :type "Float (double-precision)" :default 0.01))
  (bind __greencolor (`local._GreenColor`))
  (bind __redcolor (`local._RedColor`))
  (bind __bluecolor (`local._BlueColor`))
  (bind __colormodifier (`local._ColorModifier`))
  (set `local._RedColor` `Linear Color Input_R`)
  (set `local._BlueColor` `Linear Color Input_G`)
  (set `local._GreenColor` `Linear Color Input_B`)
  (switch `int` (`self.m_Selector`)
    (:`0`
      (set `local._GreenColor` (+ __greencolor __colormodifier))
      (if (>= (`local._GreenColor`) 1.0)
        (set `self.m_Selector` 1)))
    (:`1`
      (set `local._RedColor` (- __redcolor __colormodifier))
      (if (<= (`local._RedColor`) 0.0)
        (set `self.m_Selector` 2)))
    (:`2`
      (set `local._BlueColor` (+ __bluecolor __colormodifier))
      (if (>= (`local._BlueColor`) 1.0)
        (set `self.m_Selector` 3)))
    (:`3`
      (set `local._GreenColor` (- __greencolor __colormodifier))
      (if (<= (`local._GreenColor`) 0.0)
        (set `self.m_Selector` 4)))
    (:`4`
      (set `local._RedColor` (+ __redcolor __colormodifier))
      (if (>= (`local._RedColor`) 1.0)
        (set `self.m_Selector` 5)))
    (:`5`
      (set `local._BlueColor` (- __bluecolor __colormodifier))
      (if (<= (`local._BlueColor`) 0.0)
        (set `self.m_Selector` 0))))
  (return (make `LinearColor` (`local._RedColor`) (`local._BlueColor`) (`local._GreenColor`) `Linear Color Input_A`)))

(fn `UserConstructionScript`
  (bind _lightcolor (`self.LightColor`))
  (bind _heightofthelights (`self.HeightOfTheLights`))
  (bind _returnvalue (* -1 (+ (- 90.0 (`KismetMathLibrary.DegAtan` (/ (`self.Y_LightLocation`) (`self.HeightOfTheLights`)))) (`self.LightProjectionPosition`))))
  (bind _output_get (set `self.Y_LightLocation` (/ (`self.GapBetweenLight`) 2.0)))
  (`SceneComponent.K2_SetRelativeLocation` (`self.SpotLight01`) (`KismetMathLibrary.MakeVector` 0.0 _output_get _heightofthelights) false false)
  (`SceneComponent.K2_SetRelativeLocation` (`self.SpotLight02`) (`KismetMathLibrary.MakeVector` 0.0 (* _output_get -1.0) _heightofthelights) false false)
  (`SceneComponent.K2_SetRelativeRotation` (`self.SpotLight01`) (`KismetMathLibrary.MakeRotator` 0.0 _returnvalue -90.0) false false)
  (`SceneComponent.K2_SetRelativeRotation` (`self.SpotLight02`) (`KismetMathLibrary.MakeRotator` 0.0 _returnvalue 90.0) false false)
  (`LightComponent.SetLightColor` (`self.SpotLight01`) _lightcolor true)
  (`LightComponent.SetLightColor` (`self.SpotLight02`) _lightcolor true))