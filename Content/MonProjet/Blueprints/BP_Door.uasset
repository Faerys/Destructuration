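; Interactive door Blueprint that swings open and closed when the Use key is pressed inside its trigger box.
; DoorBoxCollision overlaps enable and disable input from player controller 0, without checking which actor overlaps.
; A FlipFlop plays or reverses a timeline that drives the yaw of DoorArrow.
; A creak sound plays as opening starts, and a closing flag triggers the shut sound when the reversed timeline finishes.
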(event `InputAction|kb_Use`
  (params (Key :type "Key Structure"))
  (bind _returnvalue (`self.K2_GetActorLocation`))
  ;[0 1 0.2705] Gère l'action Utiliser
  (:`Pressed`
    (`/Engine/EditorBlueprintResources/StandardMacros.FlipFlop`
      (:`A`
        (set `self.bDoorIsClosing` false)
        (`KismetSystemLibrary.PrintString` "Open the door")
        (`GameplayStatics.PlaySoundAtLocation` "/Game/UniversalSoundFX/Sound_Effects/DOORS_GATES_DRAWERS/DOOR_Metal_Open_Creak_stereo.DOOR_Metal_Open_Creak_stereo" _returnvalue (struct) 1.0 1.0 0.0 null null null)
        (bind (_direction _door_openning) (`Timeline|OpenDoor_TimeLine` :!label _label)
          (:`Update`
            (`SceneComponent.K2_SetRelativeRotation` (`self.DoorArrow`) (`KismetMathLibrary.MakeRotator` 0.0 0.0 _door_openning) false false))
          (:`Finished`
            (if (`self.bDoorIsClosing`)
              (`GameplayStatics.PlaySoundAtLocation` "/Game/UniversalSoundFX/Sound_Effects/DOORS_GATES_DRAWERS/DOOR_Apartment_Close_stereo.DOOR_Apartment_Close_stereo" _returnvalue (struct) 1.0 1.0 0.0 null null null)))))
      (:`B`
        (set `self.bDoorIsClosing` true)
        (`KismetSystemLibrary.PrintString` "Close the door")
        (goto _label :!via `Reverse`)))))

(event `self.DoorBoxCollision.OnComponentBeginOverlap`
  (params (OverlappedComponent :type "PrimitiveComponent Object Reference") (OtherActor :type "Actor Object Reference") (OtherComp :type "PrimitiveComponent Object Reference") (OtherBodyIndex :type Integer) (bFromSweep :type Boolean) (SweepResult :type "HitResult Structure (by ref)"))
  ;[1 0 0.9096] Gère le Trigger Box
  (`self.EnableInput` (`GameplayStatics.GetPlayerController` 0))
  (`KismetSystemLibrary.PrintString` "Player overlaps the door HitBox" true true (struct :`R` 1.0 :`G` 0.119738 :`A` 1.0)))

(event `self.DoorBoxCollision.OnComponentEndOverlap`
  (params (OverlappedComponent :type "PrimitiveComponent Object Reference") (OtherActor :type "Actor Object Reference") (OtherComp :type "PrimitiveComponent Object Reference") (OtherBodyIndex :type Integer))
  ;[1 0 0.9096] Gère le Trigger Box
  (`self.DisableInput` (`GameplayStatics.GetPlayerController` 0))
  (`KismetSystemLibrary.PrintString` "Player left the HitBox" true true (struct :`R` 1.0 :`G` 0.965879 :`A` 1.0)))

(fn `UserConstructionScript`)