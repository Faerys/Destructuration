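; BP_BigExplosion is an actor that sets off a large explosion at its location when the player presses the kb_Use0 input.
; BeginPlay enables player input; each press applies radial damage, spawns two particle effects and a sound, and shakes nearby cameras.
; DamageRadius drives damage range, effect scale and shake falloff.
; A short non-looping timer targets "Apply damage" for a second hit, while the cleared Timer handle is never assigned.
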(event `self.ReceiveBeginPlay`
  (`self.EnableInput` (`GameplayStatics.GetPlayerController` 0)))

(event `InputAction|kb_Use0`
  (params (Key :type "Key Structure"))
  (bind _damageradius (`self.DamageRadius`))
  (:`Pressed`
    (set `self.Origin` (`self.K2_GetActorLocation` self))
    (`GameplayStatics.ApplyRadialDamage` :`BaseDamage` (`self.BaseDamage`) :`Origin` (`self.Origin`) :`DamageRadius` _damageradius :`DamageCauser` null :`InstigatedByController` null)
    (`KismetSystemLibrary.K2_SetTimer` self "Apply damage" 0.03)
    (`GameplayStatics.SpawnEmitterAtLocation` "/Game/StarterContent/Particles/P_Explosion.P_Explosion" (`self.Origin`) (struct) (* (1.0 1.0 1.0) (/ _damageradius 75.0)))
    (`GameplayStatics.PlayWorldCameraShake` "/Game/IBWP3DShortStrokeAR/Blueprints/BP_ShotCameraShake.BP_ShotCameraShake_C" (`self.Origin`) 150.0 (* 10.0 _damageradius))
    (`KismetSystemLibrary.K2_ClearAndInvalidateTimerHandle` (`self.Timer`))
    (`GameplayStatics.SpawnEmitterAtLocation` "/Game/MonProjet/ParticlesSystem/Par_PlasmaBallGlass.Par_PlasmaBallGlass" (`self.Origin`) (struct) (* (1.0 1.0 1.0) (`self.DamageRadius`)))
    (`GameplayStatics.SpawnSoundAtLocation` (`self.Sound`) (`self.Origin`) (struct) 1.0 1.0 0.0 null null)))

(fn `ApplyDamage`
  (`GameplayStatics.ApplyRadialDamage` :`BaseDamage` (`self.BaseDamage`) :`Origin` (`self.Origin`) :`DamageRadius` (`self.DamageRadius`) :`DamageCauser` null :`InstigatedByController` null))

(fn `UserConstructionScript`)