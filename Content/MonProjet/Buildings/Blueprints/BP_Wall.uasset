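; BP_Wall is a building actor that builds a wall procedurally from static mesh pieces, sized by window width and height variables.
; Its construction script adds bottom and top segments with a shared scale from the window dimensions and a multiplier, offsetting the top by window height.
; When window height is positive, it adds two further pieces with their own height-derived scale.
; The event graph holds only disabled stubs.
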(fn `UserConstructionScript`
  (locals (Scale :type "Vector Structure" :default (1.0 1.0 1.0)) (ScaleMultiplyer :type "Float (double-precision)" :default 1.0) (TopWall_Location :type "Vector Structure" :default (0.0 0.0 200.0)) (BottomWall_Location :type "Vector Structure" :default (0.0 0.0 0.0)) (LeftWall_Location :type "Vector Structure") (RightWall_Location :type "Vector Structure"))
  (bind _returnvalue (/ (`self.WindowWidth`) 400.0))
  (bind _returnvalue_2 (* (`local.Scale`) (`local.ScaleMultiplyer`)))
  (bind _returnvalue_3 (* (- 2.0 (`self.WindowHeight`)) 100.0))
  (bind (_returnvalue_x _returnvalue_y _returnvalue_z) (`KismetMathLibrary.BreakVector` (* _returnvalue_2 (`local.TopWall_Location`))))
  (set `local.Scale` (`KismetMathLibrary.MakeVector` (/ (`self.WindowWidth`) 4.0) 1.0 (/ (`self.WindowHeight`) 2.0)))
  (`AddComponent|NODE_AddStaticMeshComponent-1` :`RelativeTransform` (`KismetMathLibrary.MakeTransform` (`local.BottomWall_Location`) (struct) _returnvalue_2))
  (`AddComponent|NODE_AddStaticMeshComponent-2` :`RelativeTransform` (`KismetMathLibrary.MakeTransform` (`KismetMathLibrary.MakeVector` 0.0 0.0 (+ (`self.WindowHeight`) _returnvalue_z)) (struct) _returnvalue_2))
  (if (> (`self.WindowHeight`) 0.0)
    (`AddComponent|NODE_AddStaticMeshComponent-3` :`RelativeTransform` (`KismetMathLibrary.MakeTransform` (`KismetMathLibrary.MakeVector` 0.0 0.0 _returnvalue_z) (struct) (`KismetMathLibrary.MakeVector` _returnvalue 1.0 _returnvalue_3)))
    (`AddComponent|NODE_AddStaticMeshComponent-4` :`RelativeTransform` (`KismetMathLibrary.MakeTransform` (`KismetMathLibrary.MakeVector` 0.0 0.0 _returnvalue_z) (struct) (`KismetMathLibrary.MakeVector` _returnvalue 1.0 _returnvalue_3)))))